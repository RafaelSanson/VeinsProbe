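; Spline generator actor that builds an obstacle-aware spline path between start and end locations set relative to the actor.
; GenerateSpline voxelizes the space by traces and finds a minimal path through it.
; SimplifyPath reduces it using line-of-sight traces and subdivides long edges by MaxEdgeDistance.
; Iterative AlignPath passes blend points toward locations from FindAlignedLocation before the spline is rebuilt; DestroySpline clears it.
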(event Custom|DestroySpline
  (Spline|ClearSplinePoints (Variables|Default|GetSpline) true))

(event Custom|GenerateSpline
  (Rendering|Debug|FlushPersistentDebugLines)
  (Class|PathActor|VoxelizeTrace (CallFunction|ToWorldLocation (Variables|Voxelization|Spline|GetStartLocation)) (Variables|Voxelization|Debug|GetShouldDisplayDebugInfo))
  (Class|PathActor|GetMinimalPath (CallFunction|ToWorldLocation (Variables|Voxelization|Spline|GetStartLocation)) (CallFunction|ToWorldLocation (Variables|Voxelization|Spline|GetEndLocation)) (Variables|Default|GetPath))
  (Utilities|Array|Add (Variables|Default|GetPath) (CallFunction|ToWorldLocation (Variables|Voxelization|Spline|GetEndLocation)))
  (Utilities|FlowControl|Sequence
    (:then_0
      (bind _simplifiedpath (CallFunction|SimplifyPath (Variables|Default|GetPath)))
      (Variables|Default|SetPath _simplifiedpath))
    (:then_1
      (Utilities|FlowControl|Sequence
        (:then_0
          (for _index (range 1 (Variables|Voxelization|Align|GetAlignPathIterations))
            (bind _alignedpath (CallFunction|AlignPath (Variables|Default|GetPath) (Variables|Voxelization|Align|GetAlignRadialDistance)))
            (Variables|Default|SetPath _alignedpath)))
        (:then_1
          (Utilities|Array|Insert (Variables|Default|GetPath) (CallFunction|ToWorldLocation (Variables|Voxelization|Spline|GetStartLocation)))
          (Utilities|Array|Add (Variables|Default|GetPath) (Variables|Voxelization|Spline|GetEndLocation))
          (Spline|ClearSplinePoints (Variables|Default|GetSpline) false)
          (for (_array_element _array_index) (Variables|Default|GetPath)
            (Spline|AddSplinePointatIndex (Variables|Default|GetSpline) _array_element _array_index "World" true)
            (Class|PathActor|ClearCheckedLocations)))))))

(fn ConstructionScript)

(fn DrawLinePath
  (params (@TargetArray :type Array%20of%20Vectors))
  (for _index (range 0 (- (Utilities|Array|LastIndex @TargetArray) 1))
    (bind _output_get (LocalVariables|SetLocalCurrentIndex _index))
    (LocalVariables|SetLocalNextIndex (+ _output_get 1))
    (Rendering|Debug|DrawDebugLine (Utilities|Array|Get(acopy) @TargetArray (LocalVariables|GetLocalCurrentIndex)) (Utilities|Array|Get(acopy) @TargetArray (LocalVariables|GetLocalNextIndex)) "(R=1.000000,G=0.000000,B=0.000000,A=1.000000)" 3e+01 5e+01)))

(fn SimplifyPath
  (params (@TargetArray :type Array%20of%20Vectors))
  (bind _localnewpath (LocalVariables|GetLocalNewPath))
  (Utilities|Array|Clear (LocalVariables|GetLocalNewPath))
  (bind _output_get (LocalVariables|SetLocalCurrentIndex 0))
  (LocalVariables|SetLocalNextIndex (+ _output_get 1))
  (Utilities|Array|Add (LocalVariables|GetLocalNewPath) (Utilities|Array|Get(acopy) @TargetArray (LocalVariables|GetLocalCurrentIndex)))
  (while (< (LocalVariables|GetLocalNextIndex) (Utilities|Array|LastIndex @TargetArray))
    (LocalVariables|SetLocalCurrentLocation (Utilities|Array|Get(acopy) @TargetArray (LocalVariables|GetLocalCurrentIndex)))
    (LocalVariables|SetLocalNextLocation (Utilities|Array|Get(acopy) @TargetArray (LocalVariables|GetLocalNextIndex)))
    (bind _returnvalue (Class|PathActor|LineTraceTest (LocalVariables|GetLocalCurrentLocation) (LocalVariables|GetLocalNextLocation) false))
    (LocalVariables|SetLocalHit _returnvalue)
    (if (LocalVariables|GetLocalHit)
      (LocalVariables|SetLocalCurrentIndex (- (LocalVariables|GetLocalNextIndex) 1))
      (LocalVariables|SetLocalLastPosition (Utilities|Array|Get(acopy) _localnewpath (Utilities|Array|LastIndex _localnewpath)))
      (LocalVariables|SetLocalNewPosition (Utilities|Array|Get(acopy) @TargetArray (LocalVariables|GetLocalCurrentIndex)))
      (bind _output_get_2 (LocalVariables|SetLocalNumberOfEdgesToAdd (Math|Float|Ceil (/ (Math|Vector|Distance(Vector) (LocalVariables|GetLocalLastPosition) (LocalVariables|GetLocalNewPosition)) (Variables|Voxelization|Spline|GetMaxEdgeDistance)))))
      (for _index (range 1 _output_get_2)
        (Utilities|Array|Add (LocalVariables|GetLocalNewPath) (Math|Vector|Lerp(Vector) (LocalVariables|GetLocalLastPosition) (LocalVariables|GetLocalNewPosition) (/ (Math|Conversions|ToFloat(Integer) _index) (Math|Conversions|ToFloat(Integer) (LocalVariables|GetLocalNumberOfEdgesToAdd))))))
      (else
        (Math|Integer|IncrementInt (LocalVariables|GetLocalNextIndex)))))
  (Utilities|Array|Add (LocalVariables|GetLocalNewPath) (Utilities|Array|Get(acopy) @TargetArray (Utilities|Array|LastIndex @TargetArray)))
  (return (LocalVariables|GetLocalNewPath)))

(fn AlignPath
  (params (@targetArray :type Array%20of%20Vectors) (@maxDistance :type Float%20%28single-precision%29))
  (bind _output_get (LocalVariables|SetLocalNewPath @targetArray))
  (for (_array_element _array_index) _output_get
    (bind _returnvalue (Class|PathActor|FindAlignedLocation _array_element @maxDistance))
    (Utilities|Array|SetArrayElem (LocalVariables|GetLocalNewPath) _array_index (Math|Vector|Lerp(Vector) _returnvalue _array_element (Variables|Voxelization|Align|GetAlignStrength))))
  (return (LocalVariables|GetLocalNewPath)))

(fn ToWorldLocation
  (params (A :type Vector))
  (return (+ A (Transformation|GetActorLocation))))